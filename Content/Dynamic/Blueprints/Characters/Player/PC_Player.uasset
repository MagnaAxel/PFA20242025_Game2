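; Player controller that creates the player's pawn and its companions when play begins.
; On BeginPlay it spawns PlayerClass at the named player start, possesses it and adds the IM_Player Enhanced Input mapping context.
; It then spawns each entry in CompanionClasses at a random reachable navigation point around a spot offset from the player along world X, not relative to facing.
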(event `self.ReceiveBeginPlay`
  (bind _returnvalue (`|SpawnActorFromClass` (`self.PlayerClass`) (`self.GetTransform` (`GameModeBase.K2_FindPlayerStart` (`GameplayStatics.GetGameMode`) null (`self.PlayerStart`))) "Undefined" "MultiplyWithRoot" null null))
  (`self.Possess` self _returnvalue)
  (`EnhancedInputSubsystemInterface.AddMappingContext` (pcsubsystem `EnhancedInputLocalPlayerSubsystem` self) "/Game/Dynamic/Blueprints/Characters/Player/Inputs/Maps/IM_Player.IM_Player" 0 (struct))
  (bind _result (`BlueprintSetLibrary.Set_ToArray` (`self.CompanionClasses`)))
  (for _array_element _result
    (`|SpawnActorFromClass` _array_element (`KismetMathLibrary.MakeTransform` (`NavigationSystemV1.K2_GetRandomReachablePointInRadius` (`KismetMathLibrary.MakeVector` (+ (.x (.location (`self.GetTransform` _returnvalue))) -150.0) (.y (.location (`self.GetTransform` _returnvalue))) (.z (.location (`self.GetTransform` _returnvalue)))) 200.0 null null)) "Undefined" "MultiplyWithRoot" null null)))

(fn `UserConstructionScript`)