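; BP_Collectible is an interactable pickup that gives a set of items to the player.
; On BeginPlay it resolves each entry in ItemNames through GetItem and stores the results in its Items array.
; On Interact it appends that array to the Items of the player's BPInventory, then destroys itself.
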(event `self.ReceiveBeginPlay`
  (`self.AddDataTableItems` (`self.ItemNames`)))

(event `/Game/Dynamic/Blueprints/Interfaces/BP_Interact.Interact`
  (params (Player :type "/Game/Dynamic/Blueprints/Characters/Player/BP_Player Object Reference"))
  (`KismetArrayLibrary.Array_Append` (`/Game/Dynamic/Blueprints/Characters/CharacterComponents/Inventory/BP_Inventory.Items` (`/Game/Dynamic/Blueprints/Characters/BP_Character.BP_Inventory` Player)) (`self.Items`))
  (`self.K2_DestroyActor`))

(fn `AddDataTableItems`
  (params (ItemNames :type "Array of Name"))
  (for _array_element ItemNames
    (bind _item (`/Game/Dynamic/Blueprints/Items/LF_Item.GetItem` _array_element))
    (`KismetArrayLibrary.Array_Add` (`self.Items`) _item)))

(fn `UserConstructionScript`)