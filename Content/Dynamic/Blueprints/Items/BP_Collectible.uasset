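; BP_Collectible is a world pickup that puts an item into the interacting player's inventory.
; On BeginPlay it looks up DataTableItemName in the DT_Item data table and caches the row as Item, printing a red error if the row is missing.
; Interact appends the cached Item to the player's BPInventory Items array, then destroys the actor.
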(event `self.ReceiveBeginPlay`
  (bind _datatableitemname (`self.DataTableItemName`))
  (bind _returnvalue (`|GetDataTableRow` "/Game/Dynamic/Blueprints/Items/DT_Item.DT_Item" _datatableitemname)
    (:`then`
      (set `self.Item` _returnvalue))
    (:`RowNotFound`
      (`KismetSystemLibrary.PrintString` (`KismetStringLibrary.Concat_StrStr` "Item not found : " (`KismetStringLibrary.Conv_NameToString` _datatableitemname)) true true (struct :`R` 1.0 :`A` 1.0)))))

(event `/Game/Dynamic/Blueprints/Interfaces/BP_Interact.Interact`
  (params (Player :type "/Game/Dynamic/Blueprints/Characters/Player/BP_Player Object Reference"))
  (`KismetArrayLibrary.Array_Add` (`/Game/Dynamic/Blueprints/Characters/CharacterComponents/Inventory/BP_Inventory.Items` (`/Game/Dynamic/Blueprints/Characters/BP_Character.BP_Inventory` Player)) (`self.Item`))
  (`self.K2_DestroyActor`))

(fn `UserConstructionScript`)