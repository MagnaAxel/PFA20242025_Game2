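; BP_Player is the player character Blueprint, mapping Enhanced Input actions to movement, jump, dash, interact, attack and eat.
; Capsule overlaps maintain a list of nearby actors implementing BP_Interact, and Interact sends an interface message to each.
; Move input stores a world-space direction that Dash reuses as a horizontal launch, and calls FocusThreat during combat.
; Attack, Eat and FocusThreat are defined outside these graphs, and the menu input is empty.
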(event `self.ReceiveBeginPlay`
  (`parent.ReceiveBeginPlay`))

(event `self.CapsuleComponent.OnComponentBeginOverlap`
  (params (OverlappedComponent :type "PrimitiveComponent Object Reference") (OtherActor :type "Actor Object Reference") (OtherComp :type "PrimitiveComponent Object Reference") (OtherBodyIndex :type Integer) (bFromSweep :type Boolean) (SweepResult :type "HitResult Structure (by ref)"))
  (if (`KismetSystemLibrary.DoesImplementInterface` OtherActor "/Game/Dynamic/Blueprints/Interfaces/BP_Interact.BP_Interact_C")
    (`KismetArrayLibrary.Array_AddUnique` (`self.Interactives`) OtherActor)))

(event `self.CapsuleComponent.OnComponentEndOverlap`
  (params (OverlappedComponent :type "PrimitiveComponent Object Reference") (OtherActor :type "Actor Object Reference") (OtherComp :type "PrimitiveComponent Object Reference") (OtherBodyIndex :type Integer))
  (if (`KismetSystemLibrary.DoesImplementInterface` OtherActor "/Game/Dynamic/Blueprints/Interfaces/BP_Interact.BP_Interact_C")
    (`KismetArrayLibrary.Array_RemoveItem` (`self.Interactives`) OtherActor)))

(event `EnhancedInput|/Game/Dynamic/Blueprints/Characters/Player/Inputs/Actions/IA_Move`
  (params (ActionValue :type "Vector2D Structure") (ElapsedSeconds :type "Float (double-precision)") (TriggeredSeconds :type "Float (double-precision)") (InputAction :type "InputAction Object Reference" :default "/Game/Dynamic/Blueprints/Characters/Player/Inputs/Actions/IA_Move.IA_Move"))
  (bind (_x _y) (`KismetMathLibrary.BreakVector2D` ActionValue))
  (:`Triggered`
    (bind _output_get (set `self.Direction` (`KismetMathLibrary.MakeVector` _x _y)))
    (`self.AddMovementInput` _output_get)
    (if (`self.IsInCombat`)
      (`self.FocusThreat`))))

(event `EnhancedInput|/Game/Dynamic/Blueprints/Characters/Player/Inputs/Actions/IA_Jump`
  (params (ActionValue :type Boolean) (ElapsedSeconds :type "Float (double-precision)") (TriggeredSeconds :type "Float (double-precision)") (InputAction :type "InputAction Object Reference" :default "/Game/Dynamic/Blueprints/Characters/Player/Inputs/Actions/IA_Jump.IA_Jump"))
  (:`Triggered`
    (`self.Jump`)))

(event `EnhancedInput|/Game/Dynamic/Blueprints/Characters/Player/Inputs/Actions/IA_Dash`
  (params (ActionValue :type Boolean) (ElapsedSeconds :type "Float (double-precision)") (TriggeredSeconds :type "Float (double-precision)") (InputAction :type "InputAction Object Reference" :default "/Game/Dynamic/Blueprints/Characters/Player/Inputs/Actions/IA_Dash.IA_Dash"))
  (:`Triggered`
    (`self.LaunchCharacter` (* (`self.Direction`) (1000.0 1000.0 0.0)))))

(event `EnhancedInput|/Game/Dynamic/Blueprints/Characters/Player/Inputs/Actions/IA_Interact`
  (params (ActionValue :type Boolean) (ElapsedSeconds :type "Float (double-precision)") (TriggeredSeconds :type "Float (double-precision)") (InputAction :type "InputAction Object Reference" :default "/Game/Dynamic/Blueprints/Characters/Player/Inputs/Actions/IA_Interact.IA_Interact"))
  (:`Triggered`
    (`self.Interact`)))

(event `EnhancedInput|/Game/Dynamic/Blueprints/Characters/Player/Inputs/Actions/IA_Attack`
  (params (ActionValue :type Boolean) (ElapsedSeconds :type "Float (double-precision)") (TriggeredSeconds :type "Float (double-precision)") (InputAction :type "InputAction Object Reference" :default "/Game/Dynamic/Blueprints/Characters/Player/Inputs/Actions/IA_Attack.IA_Attack"))
  (:`Triggered`
    (`self.Attack`)))

(event `EnhancedInput|/Game/Dynamic/Blueprints/Characters/Player/Inputs/Actions/IA_Eat`
  (params (ActionValue :type Boolean) (ElapsedSeconds :type "Float (double-precision)") (TriggeredSeconds :type "Float (double-precision)") (InputAction :type "InputAction Object Reference" :default "/Game/Dynamic/Blueprints/Characters/Player/Inputs/Actions/IA_Eat.IA_Eat"))
  (:`Triggered`
    (`self.Eat`)))

(event `EnhancedInput|/Game/Dynamic/Blueprints/Characters/Player/Inputs/Actions/IA_Menu`
  (params (ActionValue :type Boolean) (ElapsedSeconds :type "Float (double-precision)") (TriggeredSeconds :type "Float (double-precision)") (InputAction :type "InputAction Object Reference" :default "/Game/Dynamic/Blueprints/Characters/Player/Inputs/Actions/IA_Menu.IA_Menu")))

(fn `Interact`
  (for _array_element (`self.Interactives`)
    (message `/Game/Dynamic/Blueprints/Interfaces/BP_Interact.Interact` _array_element self)))

(fn `UserConstructionScript`
  (`parent.UserConstructionScript`))