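; Base enemy character Blueprint that exposes attack, damage, patrol route and movement speed functions, apparently for AI use.
; Attack is a placeholder that prints a debug string and immediately calls the OnAttackEnd dispatcher, while ReceiveDamage is a stub that always returns false.
; GetPatrolRoute returns the stored route, and SetMovementSpeed maps a speed state from idle to sprinting onto the character's max walk speed.
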(event `self.ReceiveBeginPlay`)

(event `Attack`
  (`KismetSystemLibrary.PrintString` "Attack Player")
  (`self.OnAttackEnd`))

(fn `GetPatrolRoute`
  (returns (PatrolRoute :type "/Game/Dynamic/Blueprints/Characters/Ennemies/AI/BP_PatrolRoute Object Reference"))
  (return (`self.PatrolRoute`)))

(fn `ReceiveDamage`
  (params (Damage :type Integer))
  (returns (IsDead :type Boolean))
  (return false))

(fn `SetMovementSpeed`
  (params (Speed :type "/Game/Dynamic/Blueprints/Characters/Ennemies/AI/Enums/E_MovementSpeed Enum" :default "NewEnumerator0"))
  (returns (SpeedValue :type "Float (double-precision)"))
  (set `CharacterMovementComponent.MaxWalkSpeed` (select `/Game/Dynamic/Blueprints/Characters/Ennemies/AI/Enums/E_MovementSpeed` Speed :`NewEnumerator1` 150.0 :`NewEnumerator2` 350.0 :`NewEnumerator3` 550.0 :!type "Float (single-precision)") (`self.CharacterMovement`))
  (return 0.0))

(fn `UserConstructionScript`
  (`parent.UserConstructionScript`))