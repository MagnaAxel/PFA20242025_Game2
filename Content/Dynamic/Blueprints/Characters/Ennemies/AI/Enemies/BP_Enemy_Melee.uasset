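; BP_Enemy_Melee is an enemy character Blueprint for the melee type, supplying combat tuning values through functions.
; It returns a fixed cooldown and a short ideal range.
; SetMovementSpeed ignores its Speed input and returns zero without changing movement.
; The event graph holds only disabled placeholder events and the construction script just calls the parent, so the Blueprint adds no other logic.
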(fn `Cooldown`
  (returns (Cooldown :type "Float (double-precision)"))
  (return 2.0))

(fn `GetIdealRange`
  (returns (AttackRadius :type "Float (double-precision)"))
  (return 100.0))

(fn `SetMovementSpeed`
  (params (Speed :type "/Game/Dynamic/Blueprints/Characters/Ennemies/AI/Enum/E_Enemy_MovementSpeed Enum" :default "NewEnumerator0"))
  (returns (SpeedValue :type "Float (double-precision)"))
  (return 0.0))

(fn `UserConstructionScript`
  (`parent.UserConstructionScript`))