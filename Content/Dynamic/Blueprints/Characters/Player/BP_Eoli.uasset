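; Eoli player character: maps Enhanced Input to movement and action calls, menu toggles on PC_Player's widget and clamped spring-arm zoom.
; Dash, attack and eat dispatchers drive an Exaltation meter: dashing and attacking raise it, eating lowers it to no less than zero.
; Each change broadcasts OnExaltationVariation, with the name switching to "Madness" above maximum.
; Capsule overlaps track BP_Interact actors, and Interact messages all of them.
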(event `self.ReceiveBeginPlay`
  (`parent.ReceiveBeginPlay`)
  (add `self.OnDashPerfomed` (delegate `AddExaltationOnDash`))
  (add `self.OnAttackPerformed` (delegate `AddExaltationOnAttack`))
  (add `self.OnEatPerformed` (delegate `SubstractExaltationOnEat`)))

(event `AddExaltationOnDash`
  (`self.AddExaltation` 5))

(event `AddExaltationOnAttack`
  (`self.AddExaltation` 3))

(event `SubstractExaltationOnEat`
  (`self.SubstractExaltation` 10))

(event `self.CapsuleComponent.OnComponentBeginOverlap`
  (params (OverlappedComponent :type "PrimitiveComponent Object Reference") (OtherActor :type "Actor Object Reference") (OtherComp :type "PrimitiveComponent Object Reference") (OtherBodyIndex :type Integer) (bFromSweep :type Boolean) (SweepResult :type "HitResult Structure (by ref)"))
  (if (`KismetSystemLibrary.DoesImplementInterface` OtherActor "/Game/Dynamic/Blueprints/Interfaces/BP_Interact.BP_Interact_C")
    (`KismetArrayLibrary.Array_AddUnique` (`self.Interactives`) OtherActor)))

(event `self.CapsuleComponent.OnComponentEndOverlap`
  (params (OverlappedComponent :type "PrimitiveComponent Object Reference") (OtherActor :type "Actor Object Reference") (OtherComp :type "PrimitiveComponent Object Reference") (OtherBodyIndex :type Integer))
  (if (`KismetSystemLibrary.DoesImplementInterface` OtherActor "/Game/Dynamic/Blueprints/Interfaces/BP_Interact.BP_Interact_C")
    (`KismetArrayLibrary.Array_RemoveItem` (`self.Interactives`) OtherActor)))

(event `EnhancedInput|/Game/Dynamic/Blueprints/Characters/Player/Inputs/Actions/IA_Move`
  (params (ActionValue :type "Vector2D Structure") (ElapsedSeconds :type "Float (double-precision)") (TriggeredSeconds :type "Float (double-precision)") (InputAction :type "InputAction Object Reference" :default "/Game/Dynamic/Blueprints/Characters/Player/Inputs/Actions/IA_Move.IA_Move"))
  (bind (_x _y) (`KismetMathLibrary.BreakVector2D` ActionValue))
  (:`Triggered`
    (`self.Move` (`KismetMathLibrary.MakeVector` _x _y))))

(event `EnhancedInput|/Game/Dynamic/Blueprints/Characters/Player/Inputs/Actions/IA_Jump`
  (params (ActionValue :type Boolean) (ElapsedSeconds :type "Float (double-precision)") (TriggeredSeconds :type "Float (double-precision)") (InputAction :type "InputAction Object Reference" :default "/Game/Dynamic/Blueprints/Characters/Player/Inputs/Actions/IA_Jump.IA_Jump"))
  (:`Triggered`
    (`self.CustomJump`)))

(event `EnhancedInput|/Game/Dynamic/Blueprints/Characters/Player/Inputs/Actions/IA_Dash`
  (params (ActionValue :type Boolean) (ElapsedSeconds :type "Float (double-precision)") (TriggeredSeconds :type "Float (double-precision)") (InputAction :type "InputAction Object Reference" :default "/Game/Dynamic/Blueprints/Characters/Player/Inputs/Actions/IA_Dash.IA_Dash"))
  (:`Triggered`
    (`self.Dash`)))

(event `EnhancedInput|/Game/Dynamic/Blueprints/Characters/Player/Inputs/Actions/IA_Interact`
  (params (ActionValue :type Boolean) (ElapsedSeconds :type "Float (double-precision)") (TriggeredSeconds :type "Float (double-precision)") (InputAction :type "InputAction Object Reference" :default "/Game/Dynamic/Blueprints/Characters/Player/Inputs/Actions/IA_Interact.IA_Interact"))
  (:`Triggered`
    (`self.Interact`)))

(event `EnhancedInput|/Game/Dynamic/Blueprints/Characters/Player/Inputs/Actions/IA_Attack`
  (params (ActionValue :type Boolean) (ElapsedSeconds :type "Float (double-precision)") (TriggeredSeconds :type "Float (double-precision)") (InputAction :type "InputAction Object Reference" :default "/Game/Dynamic/Blueprints/Characters/Player/Inputs/Actions/IA_Attack.IA_Attack"))
  (:`Triggered`
    (`self.Attack`)))

(event `EnhancedInput|/Game/Dynamic/Blueprints/Characters/Player/Inputs/Actions/IA_Eat`
  (params (ActionValue :type Boolean) (ElapsedSeconds :type "Float (double-precision)") (TriggeredSeconds :type "Float (double-precision)") (InputAction :type "InputAction Object Reference" :default "/Game/Dynamic/Blueprints/Characters/Player/Inputs/Actions/IA_Eat.IA_Eat"))
  (:`Triggered`
    (`self.Eat`)))

(event `EnhancedInput|/Game/Dynamic/Blueprints/Characters/Player/Inputs/Actions/IA_Menu`
  (params (ActionValue :type Boolean) (ElapsedSeconds :type "Float (double-precision)") (TriggeredSeconds :type "Float (double-precision)") (InputAction :type "InputAction Object Reference" :default "/Game/Dynamic/Blueprints/Characters/Player/Inputs/Actions/IA_Menu.IA_Menu"))
  (:`Triggered`
    (bind _aspc_player (cast `/Game/Dynamic/Blueprints/Characters/Player/PC_Player` (`GameplayStatics.GetPlayerController` 0)))
    (`/Game/Dynamic/Blueprints/Characters/Player/Interface/WU_Player.MenuToggle` (`/Game/Dynamic/Blueprints/Characters/Player/PC_Player.Widget` _aspc_player))))

(event `EnhancedInput|/Game/Dynamic/Blueprints/Characters/Player/Inputs/Actions/IA_Inventory`
  (params (ActionValue :type Boolean) (ElapsedSeconds :type "Float (double-precision)") (TriggeredSeconds :type "Float (double-precision)") (InputAction :type "InputAction Object Reference" :default "/Game/Dynamic/Blueprints/Characters/Player/Inputs/Actions/IA_Inventory.IA_Inventory"))
  (:`Triggered`
    (bind _aspc_player (cast `/Game/Dynamic/Blueprints/Characters/Player/PC_Player` (`GameplayStatics.GetPlayerController` 0)))
    (`/Game/Dynamic/Blueprints/Characters/Player/Interface/WU_Player.InventoryToggle` (`/Game/Dynamic/Blueprints/Characters/Player/PC_Player.Widget` _aspc_player))))

(event `EnhancedInput|/Game/Dynamic/Blueprints/Characters/Player/Inputs/Actions/IA_Option`
  (params (ActionValue :type Boolean) (ElapsedSeconds :type "Float (double-precision)") (TriggeredSeconds :type "Float (double-precision)") (InputAction :type "InputAction Object Reference" :default "/Game/Dynamic/Blueprints/Characters/Player/Inputs/Actions/IA_Option.IA_Option"))
  (:`Triggered`
    (bind _aspc_player (cast `/Game/Dynamic/Blueprints/Characters/Player/PC_Player` (`GameplayStatics.GetPlayerController` 0)))
    (`/Game/Dynamic/Blueprints/Characters/Player/Interface/WU_Player.OptionToggle` (`/Game/Dynamic/Blueprints/Characters/Player/PC_Player.Widget` _aspc_player))))

(event `EnhancedInput|/Game/Dynamic/Blueprints/Characters/Player/Inputs/Actions/IA_CameraZoom`
  (params (ActionValue :type "Float (double-precision)") (ElapsedSeconds :type "Float (double-precision)") (TriggeredSeconds :type "Float (double-precision)") (InputAction :type "InputAction Object Reference" :default "/Game/Dynamic/Blueprints/Characters/Player/Inputs/Actions/IA_CameraZoom.IA_CameraZoom"))
  (:`Triggered`
    (if (> ActionValue 0.0)
      (set `SpringArmComponent.TargetArmLength` (`KismetMathLibrary.Conv_IntToDouble` (`KismetMathLibrary.Clamp` (`KismetMathLibrary.FTrunc` (+ -10.0 (`SpringArmComponent.TargetArmLength` (`self.SpringArm`)))) 600 1200)) (`self.SpringArm`))
      (else
        (set `SpringArmComponent.TargetArmLength` (`KismetMathLibrary.Conv_IntToDouble` (`KismetMathLibrary.Clamp` (`KismetMathLibrary.FTrunc` (+ 10.0 (`SpringArmComponent.TargetArmLength` (`self.SpringArm`)))) 600 1200)) (`self.SpringArm`))))))

(fn `AddExaltation`
  (params (ToAdd :type Integer))
  (set `self.ExaltationValue` (+ (`self.ExaltationValue`) ToAdd))
  (`self.ExaltationNameSwitch`)
  (`self.OnExaltationVariation` (`self.ExaltationName`) (`self.ExaltationMaxValue`) (`self.ExaltationValue`)))

(fn `ExaltationNameSwitch`
  (if (> (`self.ExaltationValue`) (`self.ExaltationMaxValue`))
    (set `self.ExaltationName` "Madness")
    (else
      (set `self.ExaltationName` "Exaltation"))))

(fn `Interact`
  (for _array_element (`self.Interactives`)
    (message `/Game/Dynamic/Blueprints/Interfaces/BP_Interact.Interact` _array_element self)))

(fn `SubstractExaltation`
  (params (ToSubstract :type Integer))
  (bind _exaltationvalue (`self.ExaltationValue`))
  (set `self.ExaltationValue` (`KismetMathLibrary.Clamp` (- _exaltationvalue ToSubstract) 0 _exaltationvalue))
  (`self.ExaltationNameSwitch`)
  (`self.OnExaltationVariation` (`self.ExaltationName`) (`self.ExaltationMaxValue`) (`self.ExaltationValue`)))

(fn `UserConstructionScript`
  (`parent.UserConstructionScript`))