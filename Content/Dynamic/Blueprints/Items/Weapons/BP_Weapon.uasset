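; BP_Weapon is a weapon actor that deals area damage on behalf of the BP_Character it is attached to.
; On BeginPlay it loads Damage and Frequency from DT_Weapon, using its class display name as the row name.
; Attack briefly enlarges DamageArea and enables its collision to catch overlaps.
; Overlapped characters of an affiliation in the wielder's PotentialThreat receive strength-scaled damage through the BP_Damage interface.
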(event `self.ReceiveBeginPlay`
  (`parent.ReceiveBeginPlay`)
  (`self.LoadWeapon`))

(event `Attack`
  (bind _damagearea (`self.DamageArea`))
  (`PrimitiveComponent.SetCollisionEnabled` _damagearea "QueryOnly")
  (`SceneComponent.SetWorldScale3D` _damagearea (10.0 10.0 10.0))
  (`KismetSystemLibrary.Delay` 0.2)
  (`PrimitiveComponent.SetCollisionEnabled` _damagearea "NoCollision")
  (`SceneComponent.SetWorldScale3D` _damagearea (1.0 1.0 1.0)))

(event `self.DamageArea.OnComponentBeginOverlap`
  (params (OverlappedComponent :type "PrimitiveComponent Object Reference") (OtherActor :type "Actor Object Reference") (OtherComp :type "PrimitiveComponent Object Reference") (OtherBodyIndex :type Integer) (bFromSweep :type Boolean) (SweepResult :type "HitResult Structure (by ref)"))
  (if (`KismetSystemLibrary.DoesImplementInterface` OtherActor "/Game/Dynamic/Blueprints/Interfaces/BP_Damage.BP_Damage_C")
    (bind _asbp_character (cast `/Game/Dynamic/Blueprints/Characters/BP_Character` (`self.GetAttachParentActor` self)))
    (bind _asbp_character_2 (cast `/Game/Dynamic/Blueprints/Characters/BP_Character` OtherActor))
    (if (`BlueprintSetLibrary.Set_Contains` (`/Game/Dynamic/Blueprints/Characters/BP_Character.PotentialThreat` _asbp_character) (`/Game/Dynamic/Blueprints/Characters/BP_Character.Affiliation` _asbp_character_2))
      (bind _totaldamage (`self.GetTotalDamage`))
      (message `/Game/Dynamic/Blueprints/Interfaces/BP_Damage.ReceiveDamage` OtherActor _totaldamage))))

(fn `GetTotalDamage`
  (returns (TotalDamage :type Integer))
  (bind _asbp_character (cast `/Game/Dynamic/Blueprints/Characters/BP_Character` (`self.GetAttachParentActor`))
    (:`then`
      (bind _totalstrength (`/Game/Dynamic/Blueprints/Characters/BP_Character.GetTotalStrength` _asbp_character))
      (return (`KismetMathLibrary.FTrunc` (* (* (+ 100 _totalstrength) 0.01) (`self.Damage`)))))
    (:`CastFailed`
      (`KismetSystemLibrary.PrintString` "Invalid Attacker" true true (struct :`R` 1.0 :`A` 1.0))
      (return 0))))

(fn `LoadWeapon`
  (bind _returnvalue (`KismetSystemLibrary.GetClassDisplayName` (`GameplayStatics.GetObjectClass` self)))
  (bind _returnvalue_2 (`|GetDataTableRow` "/Game/Dynamic/Blueprints/Items/Weapons/DT_Weapon.DT_Weapon" (`KismetStringLibrary.Conv_StringToName` _returnvalue))
    (:`then`
      (bind (_damage _frequency) (break `/Game/Dynamic/Blueprints/Items/Weapons/ST_Weapon` _returnvalue_2))
      (set `self.Damage` _damage)
      (set `self.Frequency` _frequency))
    (:`RowNotFound`
      (`KismetSystemLibrary.PrintString` (`KismetStringLibrary.Concat_StrStr` "Character not found : " _returnvalue) true true (struct :`R` 1.0 :`A` 1.0)))))

(fn `UserConstructionScript`
  (`parent.UserConstructionScript`))