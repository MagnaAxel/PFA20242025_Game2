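; Character inventory that tracks the active weapon, ornament and food item for its owner.
; Each slot has a setter that spawns an actor of the given class at the owner's transform and stores it as the active item.
; The setters neither attach the spawned actor nor destroy the one previously held, and the event graph has no active logic.
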(fn `SetActiveFood`
  (params (Class :type "/Game/Dynamic/Blueprints/Items/Foods/BP_Food Class Reference"))
  (bind _returnvalue (`|SpawnActorFromClass` Class (`Actor.GetTransform` (`self.GetOwner`)) "Undefined" "MultiplyWithRoot" null null))
  (set `self.ActiveFood` _returnvalue))

(fn `SetActiveOrnament`
  (params (OrnamentClass :type "/Game/Dynamic/Blueprints/Items/Ornaments/BP_Ornament Class Reference"))
  (bind _returnvalue (`|SpawnActorFromClass` OrnamentClass (`Actor.GetTransform` (`self.GetOwner`)) "Undefined" "MultiplyWithRoot" null null))
  (set `self.ActiveOrnament` _returnvalue))

(fn `SetActiveWeapon`
  (params (WeaponClass :type "/Game/Dynamic/Blueprints/Items/Weapons/BP_Weapon Class Reference"))
  (bind _returnvalue (`|SpawnActorFromClass` WeaponClass (`Actor.GetTransform` (`self.GetOwner`)) "Undefined" "MultiplyWithRoot" null null))
  (set `self.ActiveWeapon` _returnvalue))