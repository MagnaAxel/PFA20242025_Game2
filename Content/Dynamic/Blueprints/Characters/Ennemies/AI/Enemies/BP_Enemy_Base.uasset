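; Base enemy character Blueprint that supplies combat and movement parameters, apparently for AI logic to query.
; Getters return a fixed cooldown, an ideal range and the assigned patrol route.
; SetMovementSpeed maps an Idle, Walking, Jogging or Sprinting state to the CharacterMovement max walk speed.
; The event graph holds only disabled placeholder events, so the class runs no logic of its own on BeginPlay, overlap or Tick.
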(fn `Cooldown`
  (returns (Cooldown :type "Float (double-precision)"))
  (return 2.0))

(fn `GetIdealRange`
  (returns (AttackRadius :type "Float (double-precision)"))
  (return 150.0))

(fn `GetPatrolRoute`
  (returns (PatrolRoute :type "/Game/Dynamic/Blueprints/Characters/Ennemies/AI/BP_PatrolRoute Object Reference"))
  (return (`self.PatrolRoute`)))

(fn `SetMovementSpeed`
  (params (Speed :type "/Game/Dynamic/Blueprints/Characters/Ennemies/AI/Enum/E_Enemy_MovementSpeed Enum" :default "NewEnumerator0"))
  (returns (SpeedValue :type "Float (double-precision)"))
  (set `CharacterMovementComponent.MaxWalkSpeed` (select `/Game/Dynamic/Blueprints/Characters/Ennemies/AI/Enum/E_Enemy_MovementSpeed` Speed :`NewEnumerator1` 150.0 :`NewEnumerator2` 350.0 :`NewEnumerator3` 550.0 :!type "Float (single-precision)") (`self.CharacterMovement`))
  (return 0.0))

(fn `UserConstructionScript`
  (`parent.UserConstructionScript`))