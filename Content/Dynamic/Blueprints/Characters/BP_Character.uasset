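; Base character that loads its stats, affiliation and sockets from DT_Character by class name, then scales movement by agility and inventory ornament bonuses.
; Overlapping hostile affiliations in CombatRange fill a threat list that toggles combat, drawing or sheathing the weapon and facing the first threat while moving.
; Move, jump, dash, attack and eat actions are gated by locker flags and BP_Cooldown objects.
; Damage is reduced by base resistance; death turns inventory into collectibles.
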(event `self.ReceiveBeginPlay`
  (`self.Bind Events`)
  (`self.LoadCharacter`)
  (`/Game/Dynamic/Blueprints/Characters/CharacterComponents/Inventory/BP_Inventory.LoadInventory` (`self.BP_Inventory`))
  (`self.SetCharacterMovement`)
  (bind _totallifepoints (`self.GetTotalLifePoints`))
  (set `self.LifePoints` _totallifepoints)
  (set `self.Direction` (`self.GetActorForwardVector` self)))

(event `Bind Events`
  (add `self.OnEnteringCombat` (delegate `EnterCombat`))
  (add `self.OnLeavingCombat` (delegate `LeaveCombat`))
  (add `self.OnDying` (delegate `Die`)))

(event `EnterCombat`
  (set `self.IsInCombat` true)
  (set `CharacterMovementComponent.bOrientRotationToMovement` false (`self.CharacterMovement`))
  (`self.DrawWeapon`))

(event `LeaveCombat`
  (set `self.IsInCombat` false)
  (set `CharacterMovementComponent.bOrientRotationToMovement` true (`self.CharacterMovement`))
  (`self.SheatheWeapon`))

(event `Die`
  (`/Game/Dynamic/Blueprints/Characters/CharacterComponents/Inventory/BP_Inventory.ToCollectible` (`self.BP_Inventory`))
  (`self.K2_DestroyActor`))

(event `self.CombatRange.OnComponentBeginOverlap`
  (params (OverlappedComponent :type "PrimitiveComponent Object Reference") (OtherActor :type "Actor Object Reference") (OtherComp :type "PrimitiveComponent Object Reference") (OtherBodyIndex :type Integer) (bFromSweep :type Boolean) (SweepResult :type "HitResult Structure (by ref)"))
  (bind _asbp_character (cast `/Game/Dynamic/Blueprints/Characters/BP_Character` OtherActor))
  (if (`BlueprintSetLibrary.Set_Contains` (`self.PotentialThreat`) (`/Game/Dynamic/Blueprints/Characters/BP_Character.Affiliation` _asbp_character))
    (`self.AddThreat` _asbp_character)))

(event `self.CombatRange.OnComponentEndOverlap`
  (params (OverlappedComponent :type "PrimitiveComponent Object Reference") (OtherActor :type "Actor Object Reference") (OtherComp :type "PrimitiveComponent Object Reference") (OtherBodyIndex :type Integer))
  (bind _asbp_character (cast `/Game/Dynamic/Blueprints/Characters/BP_Character` OtherActor))
  (if (`BlueprintSetLibrary.Set_Contains` (`self.PotentialThreat`) (`/Game/Dynamic/Blueprints/Characters/BP_Character.Affiliation` _asbp_character))
    (`self.RemoveThreat` _asbp_character)))

(event `Move`
  (params (Direction :type "Vector Structure"))
  (if (!= (`self.MoveLocker`) true)
    (bind _output_get (set `self.Direction` Direction))
    (`self.AddMovementInput` _output_get)
    (if (`self.IsInCombat`)
      (`self.FocusThreat`))))

(event `CustomJump`
  (if (!= (`self.JumpLocker`) true)
    (`self.Jump`)))

(event `Dash`
  (if (and (!= (`/Game/Dynamic/Blueprints/Characters/CharacterComponents/BP_Cooldown.IsUp` (`self.DashCooldown`)) true) (!= (`self.DashLocker`) true))
    (set `self.JumpLocker` true)
    (set `self.DashLocker` true)
    (set `self.EatLocker` true)
    (bind (_direction _dashmultiplyer) (`Timeline|DashSequence` :!via `PlayFromStart`)
      (:`Update`
        (set `MovementComponent.Velocity` (* (`self.Direction`) (`CharacterMovementComponent.MaxAcceleration` (`self.CharacterMovement`)) _dashmultiplyer) (`self.CharacterMovement`)))
      (:`Finished`
        (set `self.JumpLocker` false)
        (set `self.DashLocker` false)
        (set `self.EatLocker` false)
        (`self.OnDashPerfomed`)
        (`/Game/Dynamic/Blueprints/Characters/CharacterComponents/BP_Cooldown.Start` (`self.DashCooldown`))))))

(event `Attack`
  (bind _activeweapon (`/Game/Dynamic/Blueprints/Characters/CharacterComponents/Inventory/BP_Inventory.ActiveWeapon` (`self.BP_Inventory`)))
  (if (and (!= (`/Game/Dynamic/Blueprints/Characters/CharacterComponents/BP_Cooldown.IsUp` (`self.AttackCooldown`)) true) (!= (`self.AttackLocker`) true))
    (`/Engine/EditorBlueprintResources/StandardMacros.IsValid` _activeweapon
      (:`Is Valid`
        (`/Game/Dynamic/Blueprints/Items/Weapons/BP_Weapon.Attack` _activeweapon)
        (`self.OnAttackPerformed`)
        (`/Game/Dynamic/Blueprints/Characters/CharacterComponents/BP_Cooldown.Start` (`self.AttackCooldown`))))))

(event `Eat`
  (bind _activefood (`/Game/Dynamic/Blueprints/Characters/CharacterComponents/Inventory/BP_Inventory.ActiveFood` (`self.BP_Inventory`)))
  (if (and (!= (`/Game/Dynamic/Blueprints/Characters/CharacterComponents/BP_Cooldown.IsUp` (`self.EatCooldown`)) true) (!= (`self.EatLocker`) true))
    (`/Engine/EditorBlueprintResources/StandardMacros.IsValid` _activefood
      (:`Is Valid`
        (set `self.JumpLocker` true)
        (set `self.DashLocker` true)
        (set `self.AttackLocker` true)
        (set `self.EatLocker` true)
        (`KismetSystemLibrary.K2_SetTimerDelegate` (delegate `OnEatConsumptionFinished`) (`/Game/Dynamic/Blueprints/Items/Foods/BP_Food.Consumption` _activefood))))))

(event `OnEatConsumptionFinished`
  (`/Game/Dynamic/Blueprints/Items/Foods/BP_Food.Eat` (`/Game/Dynamic/Blueprints/Characters/CharacterComponents/Inventory/BP_Inventory.ActiveFood` (`self.BP_Inventory`)) self)
  (set `self.JumpLocker` false)
  (set `self.DashLocker` false)
  (set `self.AttackLocker` false)
  (set `self.EatLocker` false)
  (`self.OnEatPerformed`)
  (`/Game/Dynamic/Blueprints/Characters/CharacterComponents/BP_Cooldown.Start` (`self.EatCooldown`)))

(fn `AddThreat`
  (params (Threat :type "/Game/Dynamic/Blueprints/Characters/BP_Character Object Reference (by ref)"))
  (`KismetArrayLibrary.Array_AddUnique` (`self.Threats`) Threat)
  (if (== (`KismetArrayLibrary.Array_Length` (`self.Threats`)) 1)
    (`self.OnEnteringCombat`)))

(fn `DrawWeapon`
  (bind _activeweapon (`/Game/Dynamic/Blueprints/Characters/CharacterComponents/Inventory/BP_Inventory.ActiveWeapon` (`self.BP_Inventory`)))
  (if (`KismetSystemLibrary.IsValid` _activeweapon)
    (bind _returnvalue (`self.K2_AttachToComponent` _activeweapon (`self.Mesh`) (`.WeaponDrawSocketName_9_D15EDA664DCF5EAAC91AEC9F8E982524` (break `/Game/Dynamic/Blueprints/Characters/CharacterComponents/ST_SocketNames` (`self.SocketNames`))) "SnapToTarget" "KeepRelative" "KeepRelative" true))
    (if (not _returnvalue)
      (`KismetSystemLibrary.PrintString` "Unable to equip" true true (struct :`R` 1.0 :`A` 1.0) :!label _label))
    (else
      (goto _label))))

(fn `EquipFood`
  (bind _activefood (`/Game/Dynamic/Blueprints/Characters/CharacterComponents/Inventory/BP_Inventory.ActiveFood` (`self.BP_Inventory`)))
  (if (`KismetSystemLibrary.IsValid` _activefood)
    (bind _returnvalue (`self.K2_AttachToComponent` _activefood (`self.Mesh`) (`.FoodSocketName_11_4A5DE95C419156AED0035D817B568082` (break `/Game/Dynamic/Blueprints/Characters/CharacterComponents/ST_SocketNames` (`self.SocketNames`))) "SnapToTarget" "KeepRelative" "KeepRelative" true))
    (if (not _returnvalue)
      (`KismetSystemLibrary.PrintString` "Unable to equip" true true (struct :`R` 1.0 :`A` 1.0) :!label _label))
    (else
      (goto _label))))

(fn `EquipOrnament`
  (bind _activeornament (`/Game/Dynamic/Blueprints/Characters/CharacterComponents/Inventory/BP_Inventory.ActiveOrnament` (`self.BP_Inventory`)))
  (if (`KismetSystemLibrary.IsValid` _activeornament)
    (bind _returnvalue (`self.K2_AttachToComponent` _activeornament (`self.Mesh`) (`.OrnamentSocketName_10_677911AA40FF1F20A21CDDABB0251D37` (break `/Game/Dynamic/Blueprints/Characters/CharacterComponents/ST_SocketNames` (`self.SocketNames`))) "SnapToTarget" "KeepRelative" "KeepRelative" true))
    (if (not _returnvalue)
      (`KismetSystemLibrary.PrintString` "Unable to equip" true true (struct :`R` 1.0 :`A` 1.0) :!label _label))
    (else
      (goto _label))))

(fn `FocusThreat`
  (bind (_returnvalue_roll _returnvalue_pitch _returnvalue_yaw) (`KismetMathLibrary.BreakRotator` (`KismetMathLibrary.FindLookAtRotation` (`self.K2_GetActorLocation`) (`self.K2_GetActorLocation` (`|GetArrayItem` (`self.Threats`))))))
  (`self.K2_SetActorRotation` self (`KismetMathLibrary.MakeRotator` 0.0 0.0 _returnvalue_yaw) false))

(fn `GetTotalAgility`
  (returns (TotalAgility :type Integer))
  (return (`KismetMathLibrary.Clamp` (+ (`.Agility_8_F748D5E44F77279942AC998D9218D513` (break `/Game/Dynamic/Blueprints/Characters/CharacterComponents/ST_Statistics` (`self.Statistics`))) (`/Game/Dynamic/Blueprints/Items/Ornaments/BP_Ornament.AgilityModifier` (`/Game/Dynamic/Blueprints/Characters/CharacterComponents/Inventory/BP_Inventory.ActiveOrnament` (`self.BP_Inventory`)))) 0 100)))

(fn `GetTotalLifePoints`
  (returns (TotalLifePoints :type Integer))
  (bind _health (break `/Game/Dynamic/Blueprints/Characters/CharacterComponents/ST_Statistics` (`self.Statistics`)))
  (bind _activeornament (`/Game/Dynamic/Blueprints/Characters/CharacterComponents/Inventory/BP_Inventory.ActiveOrnament` (`self.BP_Inventory`)))
  (if (`KismetSystemLibrary.IsValid` _activeornament)
    (return (+ (`/Game/Dynamic/Blueprints/Items/Ornaments/BP_Ornament.HealthModifier` _activeornament) _health))
    (else
      (return _health))))

(fn `GetTotalResistance`
  (returns (TotalResistance :type Integer))
  (return (`KismetMathLibrary.Clamp` (+ (`.Resistance_10_05651FBE404AAD4E14B8BBA49E4254B0` (break `/Game/Dynamic/Blueprints/Characters/CharacterComponents/ST_Statistics` (`self.Statistics`))) (`/Game/Dynamic/Blueprints/Items/Ornaments/BP_Ornament.ResistanceModifier` (`/Game/Dynamic/Blueprints/Characters/CharacterComponents/Inventory/BP_Inventory.ActiveOrnament` (`self.BP_Inventory`)))) 0 100)))

(fn `GetTotalStrength`
  (returns (TotalStrength :type Integer))
  (return (`KismetMathLibrary.Clamp` (+ (`.Strength_9_4FF249D149BC45DFB6886C89AEFE8874` (break `/Game/Dynamic/Blueprints/Characters/CharacterComponents/ST_Statistics` (`self.Statistics`))) (`/Game/Dynamic/Blueprints/Items/Ornaments/BP_Ornament.StrengthModifier` (`/Game/Dynamic/Blueprints/Characters/CharacterComponents/Inventory/BP_Inventory.ActiveOrnament` (`self.BP_Inventory`)))) 0 100)))

(fn `LoadCharacter`
  (bind _returnvalue (`KismetSystemLibrary.GetClassDisplayName` (`GameplayStatics.GetObjectClass` self)))
  (bind _returnvalue_2 (`|GetDataTableRow` "/Game/Dynamic/Blueprints/Characters/DT_Character.DT_Character" (`KismetStringLibrary.Conv_StringToName` _returnvalue))
    (:`then`
      (bind (_charactername _charactericon _socketnames _statistics _affiliation _potentialthreat) (break `/Game/Dynamic/Blueprints/Characters/ST_Character` _returnvalue_2))
      (set `self.CharacterName` _charactername)
      (set `self.CharacterIcon` _charactericon)
      (set `self.SocketNames` _socketnames)
      (set `self.Statistics` _statistics)
      (set `self.Affiliation` _affiliation)
      (set `self.PotentialThreat` _potentialthreat))
    (:`RowNotFound`
      (`KismetSystemLibrary.PrintString` (`KismetStringLibrary.Concat_StrStr` "Character not found : " _returnvalue) true true (struct :`R` 1.0 :`A` 1.0)))))

(fn `ReceiveDamage`
  (params (Damage :type Integer))
  (returns (IsDead :type Boolean))
  (bind _output_get (set `self.LifePoints` (`KismetMathLibrary.FTrunc` (- (`self.LifePoints`) (* Damage (* (- 100 (`.Resistance_10_05651FBE404AAD4E14B8BBA49E4254B0` (break `/Game/Dynamic/Blueprints/Characters/CharacterComponents/ST_Statistics` (`self.Statistics`)))) 0.01))))))
  (bind _totallifepoints (`self.GetTotalLifePoints`))
  (`self.OnHealthVariation` _totallifepoints _output_get)
  (if (> _output_get 0)
    (return false)
    (else
      (`self.OnDying`)
      (return true))))

(fn `RemoveThreat`
  (params (Threat :type "/Game/Dynamic/Blueprints/Characters/BP_Character Object Reference (by ref)"))
  (`KismetArrayLibrary.Array_RemoveItem` (`self.Threats`) Threat)
  (if (== (`KismetArrayLibrary.Array_Length` (`self.Threats`)) 0)
    (`self.OnLeavingCombat`)))

(fn `SetCharacterMovement`
  (locals (BaseAcceleration :type "Float (double-precision)" :default 1000.0) (BaseWalkSpeed :type "Float (double-precision)" :default 600.0) (BaseJumpZVelocity :type "Float (double-precision)" :default 500.0))
  (bind _totalagility (`self.GetTotalAgility`))
  (bind _returnvalue (* (+ 100 _totalagility) 0.01))
  (set `CharacterMovementComponent.MaxAcceleration` (* (`local.BaseAcceleration`) _returnvalue) (`self.CharacterMovement`))
  (set `CharacterMovementComponent.MaxWalkSpeed` (* (`local.BaseWalkSpeed`) _returnvalue) (`self.CharacterMovement`))
  (set `CharacterMovementComponent.JumpZVelocity` (* (`local.BaseJumpZVelocity`) _returnvalue) (`self.CharacterMovement`)))

(fn `SheatheWeapon`
  (bind _activeweapon (`/Game/Dynamic/Blueprints/Characters/CharacterComponents/Inventory/BP_Inventory.ActiveWeapon` (`self.BP_Inventory`)))
  (if (`KismetSystemLibrary.IsValid` _activeweapon)
    (bind _returnvalue (`self.K2_AttachToComponent` _activeweapon (`self.Mesh`) (`.WeaponSheatheSocketName_8_F9055631433548D1B251B3B1B9D57EBC` (break `/Game/Dynamic/Blueprints/Characters/CharacterComponents/ST_SocketNames` (`self.SocketNames`))) "SnapToTarget" "KeepRelative" "KeepRelative" true))
    (if (not _returnvalue)
      (`KismetSystemLibrary.PrintString` "Unable to equip" true true (struct :`R` 1.0 :`A` 1.0) :!label _label))
    (else
      (goto _label))))

(fn `UserConstructionScript`
  ;[1 1 1] Cooldown instanciation
  (bind _returnvalue (`|GenericCreateObject` "/Game/Dynamic/Blueprints/Characters/CharacterComponents/BP_Cooldown.BP_Cooldown_C" "Dash" "/Engine/EngineResources/AICON-Green.AICON-Green" 3.0))
  (set `self.DashCooldown` _returnvalue)
  (bind _returnvalue_2 (`|GenericCreateObject` "/Game/Dynamic/Blueprints/Characters/CharacterComponents/BP_Cooldown.BP_Cooldown_C" "Attack" "/Engine/EditorResources/Ai_Spawnpoint.Ai_Spawnpoint" 0.2))
  (set `self.AttackCooldown` _returnvalue_2)
  (bind _returnvalue_3 (`|GenericCreateObject` "/Game/Dynamic/Blueprints/Characters/CharacterComponents/BP_Cooldown.BP_Cooldown_C" "Eat" "/Engine/MobileResources/HUD/AnalogHat.AnalogHat" 10.0))
  (set `self.EatCooldown` _returnvalue_3))