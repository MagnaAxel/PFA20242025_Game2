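; Character inventory component that holds an item list plus one active weapon, ornament and food actor.
; SetActiveItem routes by item class to setters that return the previous item to the list, spawn the new actor and update the owning character.
; LoadInventory fills it from data tables keyed by class name, while SaveInventory returns a class-based snapshot struct.
; ToCollectible destroys the active actors and spawns a BP_Collectible holding all items at the owner's transform.
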(fn `LoadInventory`
  (bind _returnvalue (`KismetSystemLibrary.GetClassDisplayName` (`GameplayStatics.GetObjectClass` (`self.GetOwner`))))
  (bind _returnvalue_2 (`|GetDataTableRow` "/Game/Dynamic/Blueprints/Characters/CharacterComponents/Inventory/DT_InventoryImage.DT_InventoryImage" (`KismetStringLibrary.Conv_StringToName` _returnvalue))
    (:`then`
      (bind (_activeweapon _activeornament _activefood _items) (break `/Game/Dynamic/Blueprints/Characters/CharacterComponents/Inventory/ST_InventoryImage` _returnvalue_2))
      (`self.SetActiveWeapon` _activeweapon)
      (`self.SetActiveOrnament` _activeornament)
      (`self.SetActiveFood` _activefood)
      (for _array_element _items
        (bind _returnvalue_3 (`KismetSystemLibrary.GetClassDisplayName` _array_element))
        (bind _returnvalue_4 (`|GetDataTableRow` "/Game/Dynamic/Blueprints/Items/DT_Item.DT_Item" (`KismetStringLibrary.Conv_StringToName` _returnvalue_3))
          (:`then`
            (`KismetArrayLibrary.Array_Add` (`self.Items`) _returnvalue_4))
          (:`RowNotFound`
            (`KismetSystemLibrary.PrintString` (`KismetStringLibrary.Concat_StrStr` "Item not found : " _returnvalue_3) true true (struct :`R` 1.0 :`A` 1.0))))))
    (:`RowNotFound`
      (`KismetSystemLibrary.PrintString` (`KismetStringLibrary.Concat_StrStr` "InventoryImage not found : " _returnvalue) true true (struct :`R` 1.0 :`A` 1.0)))))

(fn `SaveInventory`
  (returns (InventoryImage :type "/Game/Dynamic/Blueprints/Characters/CharacterComponents/Inventory/ST_InventoryImage Structure"))
  (locals (ItemClasses :type "Array of /Game/Dynamic/Blueprints/Items/BP_Item Class Reference"))
  (for _array_element (`self.Items`)
    (`KismetArrayLibrary.Array_Add` (`local.ItemClasses`) (`.class_31_AFDC24EA4C201401CC469DADBDF6D8EC` (break `/Game/Dynamic/Blueprints/Items/ST_Item` _array_element))))
  (return (make `/Game/Dynamic/Blueprints/Characters/CharacterComponents/Inventory/ST_InventoryImage` (`GameplayStatics.GetObjectClass` (`self.ActiveWeapon`)) (`GameplayStatics.GetObjectClass` (`self.ActiveOrnament`)) (`GameplayStatics.GetObjectClass` (`self.ActiveFood`)) (`local.ItemClasses`))))

(fn `SetActiveFood`
  (params (Class :type "/Game/Dynamic/Blueprints/Items/Foods/BP_Food Class Reference"))
  (`/Engine/EditorBlueprintResources/StandardMacros.IsValid` (`self.ActiveFood`)
    (:`Is Valid`
      (`KismetArrayLibrary.Array_Add` (`self.Items`) (`/Game/Dynamic/Blueprints/Items/BP_Item.Item` (`self.ActiveFood`)))
      (`Actor.K2_DestroyActor` (`self.ActiveFood`)))
    (:`Is Not Valid`
      _))
  (bind _returnvalue (`|SpawnActorFromClass` Class (`Actor.GetTransform` (`self.GetOwner`)) "Undefined" "MultiplyWithRoot" null null))
  (set `self.ActiveFood` _returnvalue)
  (bind _asbp_character (cast `/Game/Dynamic/Blueprints/Characters/BP_Character` (`self.GetOwner`)))
  (`/Game/Dynamic/Blueprints/Characters/BP_Character.EquipFood` _asbp_character))

(fn `SetActiveItem`
  (params (Item :type "/Game/Dynamic/Blueprints/Items/ST_Item Structure (by ref)"))
  (bind (_name _icon _class) (break `/Game/Dynamic/Blueprints/Items/ST_Item` Item))
  (bind _asbp_weapon (castclass `/Game/Dynamic/Blueprints/Items/Weapons/BP_Weapon` _class)
    (:`then`
      (`self.SetActiveWeapon` _asbp_weapon))
    (:`CastFailed`
      (bind _asbp_ornament (castclass `/Game/Dynamic/Blueprints/Items/Ornaments/BP_Ornament` _class)
        (:`then`
          (`self.SetActiveOrnament` _asbp_ornament))
        (:`CastFailed`
          (bind _asbp_food (castclass `/Game/Dynamic/Blueprints/Items/Foods/BP_Food` _class))
          (`self.SetActiveFood` _asbp_food))))))

(fn `SetActiveOrnament`
  (params (OrnamentClass :type "/Game/Dynamic/Blueprints/Items/Ornaments/BP_Ornament Class Reference"))
  (`/Engine/EditorBlueprintResources/StandardMacros.IsValid` (`self.ActiveOrnament`)
    (:`Is Valid`
      (`KismetArrayLibrary.Array_Add` (`self.Items`) (`/Game/Dynamic/Blueprints/Items/BP_Item.Item` (`self.ActiveOrnament`)))
      (`Actor.K2_DestroyActor` (`self.ActiveOrnament`)))
    (:`Is Not Valid`
      _))
  (bind _returnvalue (`|SpawnActorFromClass` OrnamentClass (`Actor.GetTransform` (`self.GetOwner`)) "Undefined" "MultiplyWithRoot" null null))
  (set `self.ActiveOrnament` _returnvalue)
  (bind _asbp_character (cast `/Game/Dynamic/Blueprints/Characters/BP_Character` (`self.GetOwner`)))
  (`/Game/Dynamic/Blueprints/Characters/BP_Character.EquipOrnament` _asbp_character))

(fn `SetActiveWeapon`
  (params (WeaponClass :type "/Game/Dynamic/Blueprints/Items/Weapons/BP_Weapon Class Reference"))
  (`/Engine/EditorBlueprintResources/StandardMacros.IsValid` (`self.ActiveWeapon`)
    (:`Is Valid`
      (`KismetArrayLibrary.Array_Add` (`self.Items`) (`/Game/Dynamic/Blueprints/Items/BP_Item.Item` (`self.ActiveWeapon`)))
      (`Actor.K2_DestroyActor` (`self.ActiveWeapon`)))
    (:`Is Not Valid`
      _))
  (bind _returnvalue (`|SpawnActorFromClass` WeaponClass (`Actor.GetTransform` (`self.GetOwner`)) "Undefined" "MultiplyWithRoot" null null))
  (set `self.ActiveWeapon` _returnvalue)
  (bind _asbp_character (cast `/Game/Dynamic/Blueprints/Characters/BP_Character` (`self.GetOwner`)))
  (if (`/Game/Dynamic/Blueprints/Characters/BP_Character.IsInCombat` _asbp_character)
    (`/Game/Dynamic/Blueprints/Characters/BP_Character.DrawWeapon` _asbp_character)
    (else
      (`/Game/Dynamic/Blueprints/Characters/BP_Character.SheatheWeapon` _asbp_character))))

(fn `ToCollectible`
  (locals (ItemList :type "Array of /Game/Dynamic/Blueprints/Items/ST_Item Structure"))
  (`KismetArrayLibrary.Array_Add` (`local.ItemList`) (`/Game/Dynamic/Blueprints/Items/BP_Item.Item` (`self.ActiveWeapon`)))
  (`Actor.K2_DestroyActor` (`self.ActiveWeapon`))
  (`KismetArrayLibrary.Array_Add` (`local.ItemList`) (`/Game/Dynamic/Blueprints/Items/BP_Item.Item` (`self.ActiveOrnament`)))
  (`Actor.K2_DestroyActor` (`self.ActiveOrnament`))
  (`KismetArrayLibrary.Array_Add` (`local.ItemList`) (`/Game/Dynamic/Blueprints/Items/BP_Item.Item` (`self.ActiveFood`)))
  (`Actor.K2_DestroyActor` (`self.ActiveFood`))
  (`KismetArrayLibrary.Array_Append` (`local.ItemList`) (`self.Items`))
  (bind _returnvalue (`|SpawnActorFromClass` "/Game/Dynamic/Blueprints/Items/Collectible/BP_Collectible.BP_Collectible_C" (`Actor.GetTransform` (`self.GetOwner` self)) "Undefined" "MultiplyWithRoot" null null))
  (set `/Game/Dynamic/Blueprints/Items/Collectible/BP_Collectible.Items` (`local.ItemList`) _returnvalue))