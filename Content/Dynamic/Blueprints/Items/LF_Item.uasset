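; Blueprint function library for looking up item definitions by name in the DT_Item data table.
; GetItem returns the matching row, printing a red error with the name when it is missing.
; GetWeapon, GetOrnament and GetFood build on GetItem, casting the row's Class to BP_Weapon, BP_Ornament or BP_Food and printing a red error when the type does not match.
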(fn `GetFood`
  (params (ItemName :type Name))
  (returns (Food :type "/Game/Dynamic/Blueprints/Items/Foods/BP_Food Class Reference"))
  (bind _item (`self.GetItem` ItemName))
  (bind _asbp_food (castclass `/Game/Dynamic/Blueprints/Items/Foods/BP_Food` (`.class_31_AFDC24EA4C201401CC469DADBDF6D8EC` (break `/Game/Dynamic/Blueprints/Items/ST_Item` _item)))
    (:`then`
      (return _asbp_food))
    (:`CastFailed`
      (`KismetSystemLibrary.PrintString` null "Not a food" true true (struct :`R` 1.0 :`A` 1.0))
      (return null))))

(fn `GetItem`
  (params (ItemName :type Name))
  (returns (Item :type "/Game/Dynamic/Blueprints/Items/ST_Item Structure"))
  (bind _returnvalue (`|GetDataTableRow` "/Game/Dynamic/Blueprints/Items/DT_Item.DT_Item" ItemName)
    (:`then`
      (return _returnvalue))
    (:`RowNotFound`
      (`KismetSystemLibrary.PrintString` null (`KismetStringLibrary.Concat_StrStr` "Item not found : " (`KismetStringLibrary.Conv_NameToString` ItemName)) true true (struct :`R` 1.0 :`A` 1.0))
      (return))))

(fn `GetOrnament`
  (params (ItemName :type Name))
  (returns (Ornament :type "/Game/Dynamic/Blueprints/Items/Ornaments/BP_Ornament Class Reference"))
  (bind _item (`self.GetItem` ItemName))
  (bind _asbp_ornament (castclass `/Game/Dynamic/Blueprints/Items/Ornaments/BP_Ornament` (`.class_31_AFDC24EA4C201401CC469DADBDF6D8EC` (break `/Game/Dynamic/Blueprints/Items/ST_Item` _item)))
    (:`then`
      (return _asbp_ornament))
    (:`CastFailed`
      (`KismetSystemLibrary.PrintString` null "Not an ornament" true true (struct :`R` 1.0 :`A` 1.0))
      (return null))))

(fn `GetWeapon`
  (params (ItemName :type Name))
  (returns (Weapon :type "/Game/Dynamic/Blueprints/Items/Weapons/BP_Weapon Class Reference"))
  (bind _item (`self.GetItem` ItemName))
  (bind _asbp_weapon (castclass `/Game/Dynamic/Blueprints/Items/Weapons/BP_Weapon` (`.class_31_AFDC24EA4C201401CC469DADBDF6D8EC` (break `/Game/Dynamic/Blueprints/Items/ST_Item` _item)))
    (:`then`
      (return _asbp_weapon))
    (:`CastFailed`
      (`KismetSystemLibrary.PrintString` null "Not a weapon" true true (struct :`R` 1.0 :`A` 1.0))
      (return null))))