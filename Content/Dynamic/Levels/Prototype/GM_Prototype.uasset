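; Prototype game mode that spawns the player character and its companions when play begins.
; Each actor spawns at the player start found by the name "default_" plus its class display name.
; Companions from the configured class collection are registered in the player actor's Companions list.
; The first player controller then possesses the player actor and, as PC_Player, is initialized.
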(event `self.ReceiveBeginPlay`
  (bind _returnvalue (`GameplayStatics.GetPlayerController` 0))
  (bind _playerclass (`self.PlayerClass`))
  (bind _returnvalue_2 (`|SpawnActorFromClass` _playerclass (`self.GetTransform` (`self.K2_FindPlayerStart` (`GameplayStatics.GetPlayerController` 0) (`KismetStringLibrary.Concat_StrStr` "default_" (`KismetSystemLibrary.GetClassDisplayName` _playerclass)))) "Undefined" "MultiplyWithRoot" null null))
  (`self.SpawnCompanions` _returnvalue_2)
  (`Controller.Possess` _returnvalue _returnvalue_2)
  (bind _aspc_player (cast `/Game/Dynamic/Blueprints/Characters/Player/PC_Player` _returnvalue))
  (`/Game/Dynamic/Blueprints/Characters/Player/PC_Player.Initialize` _aspc_player))

(event `SpawnCompanions`
  (params (Eoli :type "/Game/Dynamic/Blueprints/Characters/Player/BP_Eoli Object Reference (by ref)"))
  (bind _result (`BlueprintSetLibrary.Set_ToArray` (`self.CompanionClasses`)))
  (for _array_element _result
    (bind _returnvalue (`|SpawnActorFromClass` _array_element (`self.GetTransform` (`self.K2_FindPlayerStart` (`GameplayStatics.GetPlayerController` 0) (`KismetStringLibrary.Concat_StrStr` "default_" (`KismetSystemLibrary.GetClassDisplayName` _array_element)))) "Undefined" "MultiplyWithRoot" null null))
    (`KismetArrayLibrary.Array_AddUnique` (`/Game/Dynamic/Blueprints/Characters/Player/BP_Eoli.Companions` Eoli) _returnvalue)))

(fn `UserConstructionScript`)