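; BP_Food is a food item that restores a character's health when eaten.
; Its Eat event adds the Regeneration amount to the character's Health, clamped between zero and that character's total health.
; It then fires the character's OnHealthVariation call with the total and current life points, and destroys the food actor.
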(event `Eat`
  (params (Character :type "/Game/Dynamic/Blueprints/Characters/BP_Character Object Reference"))
  (bind _totallifepoints (`/Game/Dynamic/Blueprints/Characters/BP_Character.GetTotalHealth` Character))
  (bind _output_get (set `/Game/Dynamic/Blueprints/Characters/BP_Character.Health` (`KismetMathLibrary.Clamp` (+ (`/Game/Dynamic/Blueprints/Characters/BP_Character.Health` Character) (`self.Regeneration`)) 0 _totallifepoints) Character))
  (`/Game/Dynamic/Blueprints/Characters/BP_Character.OnHealthVariation` Character _totallifepoints _output_get)
  (`self.K2_DestroyActor`))

(fn `UserConstructionScript`
  (`parent.UserConstructionScript`))