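; BP_Exaltation tracks the player's Exaltation value, which other logic can add to or subtract from.
; Each change re-evaluates the state name, which becomes "Madness" while the value exceeds its maximum and "Exaltation" otherwise.
; It then fires the OnExaltationVariation dispatcher with the name, maximum and current value.
; The value is never clamped, so it can pass the maximum or drop below zero.
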(fn `AddExaltation`
  (params (ToAdd :type Integer))
  (set `self.ExaltationValue` (+ (`self.ExaltationValue`) ToAdd))
  (`self.ExaltationNameSwitch`)
  (`self.OnExaltationVariation` (`self.ExaltationName`) (`self.ExaltationMaxValue`) (`self.ExaltationValue`)))

(fn `ExaltationNameSwitch`
  (if (> (`self.ExaltationValue`) (`self.ExaltationMaxValue`))
    (set `self.ExaltationName` "Madness")
    (else
      (set `self.ExaltationName` "Exaltation"))))

(fn `SubstractExaltation`
  (params (ToSubstract :type Integer))
  (set `self.ExaltationValue` (- (`self.ExaltationValue`) ToSubstract))
  (`self.ExaltationNameSwitch`)
  (`self.OnExaltationVariation` (`self.ExaltationName`) (`self.ExaltationMaxValue`) (`self.ExaltationValue`)))